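; Castle gate actor that opens once the player's third-person character holds enough juggling balls.
; On BeginPlay it caches the player character and starts a looping timer that periodically polls the character's JugglingBallsAmount.
; When the threshold is met, it snaps the gate mesh downward without interpolation, then pauses the timer after a short delay.
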(event `self.ReceiveBeginPlay`
  (bind _asbp_third_person_character (cast `/Game/ThirdPerson/Blueprints/BP_ThirdPersonCharacter` (`GameplayStatics.GetPlayerCharacter` 0)))
  (set `self.Player` _asbp_third_person_character)
  (bind _returnvalue (`KismetSystemLibrary.K2_SetTimerDelegate` (delegate `Open Gate`) 2.0 true))
  (set `self.Gate Timer` _returnvalue))

(event `Open Gate`
  (if (>= (`/Game/ThirdPerson/Blueprints/BP_ThirdPersonCharacter.JugglingBallsAmount` (`self.Player`)) 2)
    (`SceneComponent.K2_SetRelativeLocation` (`self.gate`) (0.0 0.0 -500.0) false false)
    (`KismetSystemLibrary.Delay` 2.0)
    (`KismetSystemLibrary.K2_PauseTimerHandle` (`self.Gate Timer`))))

(fn `UserConstructionScript`)