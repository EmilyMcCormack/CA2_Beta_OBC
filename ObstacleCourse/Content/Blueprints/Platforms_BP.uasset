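; Crumbling platform Blueprint that breaks away under the third-person character and later reappears.
; Box overlap plays a break sound for any actor, then, for the character only, swaps to a grime material and after a short delay hides the platform and disables its collision.
; When any overlap ends, another delay precedes restoring the original material, visibility and collision.
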(event `self.Box.OnComponentBeginOverlap`
  (params (OverlappedComponent :type "PrimitiveComponent Object Reference") (OtherActor :type "Actor Object Reference") (OtherComp :type "PrimitiveComponent Object Reference") (OtherBodyIndex :type Integer) (bFromSweep :type Boolean) (SweepResult :type "HitResult Structure (by ref)"))
  (`GameplayStatics.PlaySound2D` "/Game/Audio_Files/PlatformBreak.PlatformBreak" 1.0 1.0 0.0 null null)
  (cast `/Game/ThirdPerson/Blueprints/BP_ThirdPersonCharacter` OtherActor)
  (`PrimitiveComponent.SetMaterial` (`self.Platform`) 0 "/Game/StarterContent/Materials/M_Concrete_Grime.M_Concrete_Grime")
  (`KismetSystemLibrary.Delay` 0.8)
  (`SceneComponent.SetVisibility` (`self.Platform`) false false)
  (`PrimitiveComponent.SetCollisionEnabled` (`self.Platform`) "NoCollision"))

(event `self.Box.OnComponentEndOverlap`
  (params (OverlappedComponent :type "PrimitiveComponent Object Reference") (OtherActor :type "Actor Object Reference") (OtherComp :type "PrimitiveComponent Object Reference") (OtherBodyIndex :type Integer))
  (`KismetSystemLibrary.Delay` 0.5)
  (`PrimitiveComponent.SetMaterial` (`self.Platform`) 0 "/Game/PlatForm.PlatForm")
  (`SceneComponent.SetVisibility` (`self.Platform`) true false)
  (`PrimitiveComponent.SetCollisionEnabled` (`self.Platform`) "QueryAndPhysics"))

(fn `UserConstructionScript`)