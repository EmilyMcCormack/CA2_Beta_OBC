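; Castle door actor that swings open once the player holds at least one juggling ball.
; BeginPlay caches the third-person character, checks immediately, then repeats the check on a looping timer rather than using overlap or Tick.
; When the check passes, a timeline lerps the static mesh's relative yaw through a quarter turn; nothing in the graph closes it again.
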(event `OpenDoor2`
  (if (>= (`/Game/ThirdPerson/Blueprints/BP_ThirdPersonCharacter.JugglingBallsAmount` (`self.player`)) 1)
    (bind (_direction _newtrack_0) (`Timeline|OpenDoor`)
      (:`Update`
        (`SceneComponent.K2_SetRelativeRotation` (`self.StaticMesh`) (`KismetMathLibrary.MakeRotator` 0.0 0.0 (`KismetMathLibrary.Lerp` 0.0 -90.0 _newtrack_0)) false false)))))

(event `self.ReceiveBeginPlay`
  (bind _asbp_third_person_character (cast `/Game/ThirdPerson/Blueprints/BP_ThirdPersonCharacter` (`GameplayStatics.GetPlayerCharacter` 0)))
  (set `self.player` _asbp_third_person_character)
  (`KismetSystemLibrary.K2_SetTimerDelegate` (delegate `OpenDoor2`) 10.0 true)
  (`self.OpenDoor2`))

(fn `UserConstructionScript`)