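; A functional test that checks whether the player character dies when its health is decreased.
; PrepareTest caches the player pawn as a BP_ThirdPersonCharacter.
; StartTest sets Health to 50, calls DecreaseHealth once, then asserts the Dead flag and finishes as succeeded or failed with a message.
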(event `self.ReceivePrepareTest`
  (bind _asbp_third_person_character (cast `/Game/ThirdPerson/Blueprints/BP_ThirdPersonCharacter` (`GameplayStatics.GetPlayerCharacter` 0)))
  (set `self.Dimples` _asbp_third_person_character))

(event `self.ReceiveStartTest`
  (bind _dimples (`self.Dimples`))
  (set `/Game/ThirdPerson/Blueprints/BP_ThirdPersonCharacter.Health` 50 _dimples)
  (`/Game/ThirdPerson/Blueprints/BP_ThirdPersonCharacter.Decrease_Health` _dimples)
  (bind _returnvalue (`self.AssertTrue` (`/Game/ThirdPerson/Blueprints/BP_ThirdPersonCharacter.Dead` _dimples)))
  (if _returnvalue
    (`self.FinishTest` "Succeeded" "You died!")
    (else
      (`self.FinishTest` "Failed" "You're still alive"))))

(fn `UserConstructionScript`)