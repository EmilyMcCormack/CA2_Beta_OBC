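; Functional test that checks the player character's juggling ball counter increases correctly.
; PrepareTest casts player character 0 to BP_ThirdPersonCharacter and caches it as Dimples.
; StartTest zeroes JugglingBallsAmount, calls IncreaseJugglingBallAmount, asserts the count equals one, and finishes as succeeded or failed.
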(event `self.ReceivePrepareTest`
  (bind _asbp_third_person_character (cast `/Game/ThirdPerson/Blueprints/BP_ThirdPersonCharacter` (`GameplayStatics.GetPlayerCharacter` 0)))
  (set `self.Dimples` _asbp_third_person_character))

(event `self.ReceiveStartTest`
  (bind _dimples (`self.Dimples`))
  (set `/Game/ThirdPerson/Blueprints/BP_ThirdPersonCharacter.JugglingBallsAmount` 0 _dimples)
  (`/Game/ThirdPerson/Blueprints/BP_ThirdPersonCharacter.Increase_JugglingBall_Amount` _dimples)
  (bind _returnvalue (`self.AssertValue_Int` (`/Game/ThirdPerson/Blueprints/BP_ThirdPersonCharacter.JugglingBallsAmount` _dimples) "Equal_To" 1))
  (if _returnvalue
    (`self.FinishTest` "Succeeded" "yippee")
    (else
      (`self.FinishTest` "Failed" ":("))))

(fn `UserConstructionScript`)