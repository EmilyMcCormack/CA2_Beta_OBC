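; Functional test that checks whether a third-person character's health drops to 50 after being damaged.
; It spawns a test character at SpawnPoint with full health, then spawns an actor high above it and waits a second.
; Before the check, it overwrites the test character's Health with that of the cached player character, so the result actually reflects the player's health, which is also the failure message.
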(event `self.ReceivePrepareTest`
  (bind _asbp_third_person_character (cast `/Game/ThirdPerson/Blueprints/BP_ThirdPersonCharacter` (`GameplayStatics.GetPlayerCharacter` 0)))
  (set `self.Player` _asbp_third_person_character))

(event `self.ReceiveStartTest`
  (bind _test_character (`self.Test_Character`))
  (bind (_returnvalue_x _returnvalue_y _returnvalue_z) (`KismetMathLibrary.BreakVector` (`self.K2_GetActorLocation` (`self.Test_Character`))))
  (bind _health (`/Game/ThirdPerson/Blueprints/BP_ThirdPersonCharacter.Health` (`self.Player`)))
  (bind _returnvalue (`|SpawnActorFromClass` "/Game/ThirdPerson/Blueprints/BP_ThirdPersonCharacter.BP_ThirdPersonCharacter_C" (`KismetMathLibrary.MakeTransform` (`self.K2_GetActorLocation` (`self.Spawn_Point`))) "Undefined" "MultiplyWithRoot" null null))
  (bind _output_get (set `self.Test_Character` _returnvalue))
  (set `/Game/ThirdPerson/Blueprints/BP_ThirdPersonCharacter.Health` 100 _output_get)
  (`|SpawnActorFromClass` "/Game/Blueprints/FallingObject_BP.FallingObject_BP_C" (`KismetMathLibrary.MakeTransform` (`KismetMathLibrary.MakeVector` _returnvalue_x _returnvalue_y (+ _returnvalue_z 760.0))) "Undefined" "MultiplyWithRoot" null null)
  (`KismetSystemLibrary.Delay` 1.0)
  (set `/Game/ThirdPerson/Blueprints/BP_ThirdPersonCharacter.Health` _health _test_character)
  (if (== (`/Game/ThirdPerson/Blueprints/BP_ThirdPersonCharacter.Health` _test_character) 50)
    (`self.FinishTest` "Succeeded" "Character damaged correctly")
    (else
      (`self.FinishTest` "Failed" (`KismetStringLibrary.Conv_IntToString` _health)))))

(fn `UserConstructionScript`)