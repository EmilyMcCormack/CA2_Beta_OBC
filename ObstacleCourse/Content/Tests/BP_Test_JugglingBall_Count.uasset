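; Functional test that checks whether picking up a JugglingBalls_BP gives a count of one juggling ball.
; PrepareTest caches the player's third-person character; StartTest spawns an AI-controlled test character and a ball at two spawn points, then issues AIMoveTo toward the ball.
; Three seconds after issuing the move, it copies the player's JugglingBallsAmount onto the test character, so pass or fail depends on the player's count.
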(event `self.ReceivePrepareTest`
  (bind _asbp_third_person_character (cast `/Game/ThirdPerson/Blueprints/BP_ThirdPersonCharacter` (`GameplayStatics.GetPlayerCharacter` 0)))
  (set `self.Player` _asbp_third_person_character))

(event `self.ReceiveStartTest`
  (bind _test_character (`self.Test_Character`))
  (bind _jugglingballsamount (`/Game/ThirdPerson/Blueprints/BP_ThirdPersonCharacter.JugglingBallsAmount` _test_character))
  (bind _returnvalue (`|SpawnActorFromClass` "/Game/ThirdPerson/Blueprints/BP_ThirdPersonCharacter.BP_ThirdPersonCharacter_C" (`KismetMathLibrary.MakeTransform` (`self.K2_GetActorLocation` (`self.Spawn_Point`))) "Undefined" "MultiplyWithRoot" null null))
  (bind _output_get (set `self.Test_Character` _returnvalue))
  (set `/Game/ThirdPerson/Blueprints/BP_ThirdPersonCharacter.JugglingBallsAmount` 0 _output_get)
  (`Pawn.SpawnDefaultController` (`self.Test_Character`))
  (bind _returnvalue_2 (`|SpawnActorFromClass` "/Game/Blueprints/JugglingBalls_BP.JugglingBalls_BP_C" (`KismetMathLibrary.MakeTransform` (`self.K2_GetActorLocation` (`self.Spawn_Point_2`))) "Undefined" "MultiplyWithRoot" null null))
  (`|AIMoveTo` (`self.Test_Character`) (`self.K2_GetActorLocation` _returnvalue_2) null
    (:`then`
      (`KismetSystemLibrary.Delay` 3.0)
      (set `/Game/ThirdPerson/Blueprints/BP_ThirdPersonCharacter.JugglingBallsAmount` (`/Game/ThirdPerson/Blueprints/BP_ThirdPersonCharacter.JugglingBallsAmount` (`self.Player`)) _test_character)
      (if (== _jugglingballsamount 1)
        (`self.FinishTest` "Succeeded" "Ball")
        (else
          (`self.FinishTest` "Failed" (`KismetStringLibrary.Conv_IntToString` _jugglingballsamount)))))))

(fn `UserConstructionScript`)