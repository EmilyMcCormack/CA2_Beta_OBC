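; Functional test Blueprint that checks whether the third-person character's IncreaseHealth function raises health by the expected amount.
; PrepareTest casts the player pawn to BP_ThirdPersonCharacter and caches it.
; StartTest sets a known starting health, calls IncreaseHealth, asserts the resulting value, and finishes the test as succeeded or failed with a message.
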(event `self.ReceivePrepareTest`
  (bind _asbp_third_person_character (cast `/Game/ThirdPerson/Blueprints/BP_ThirdPersonCharacter` (`GameplayStatics.GetPlayerCharacter` 0)))
  (set `self.Dimples` _asbp_third_person_character))

(event `self.ReceiveStartTest`
  (bind _dimples (`self.Dimples`))
  (set `/Game/ThirdPerson/Blueprints/BP_ThirdPersonCharacter.Health` 50 _dimples)
  (`/Game/ThirdPerson/Blueprints/BP_ThirdPersonCharacter.Increase_Health` _dimples)
  (bind _returnvalue (`self.AssertValue_Int` (`/Game/ThirdPerson/Blueprints/BP_ThirdPersonCharacter.Health` _dimples) "Equal_To" 75))
  (if _returnvalue
    (`self.FinishTest` "Succeeded" "Health increased")
    (else
      (`self.FinishTest` "Failed" "Health NOT increased"))))

(fn `UserConstructionScript`)