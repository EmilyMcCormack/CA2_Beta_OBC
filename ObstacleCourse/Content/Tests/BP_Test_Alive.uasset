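; Functional test that checks the third-person character stays alive after its health increases.
; PrepareTest caches player zero's BP_ThirdPersonCharacter.
; StartTest sets its health to full, calls IncreaseHealth and asserts that Alive is true.
; The test then finishes as succeeded or failed based on that result.
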(event `self.ReceivePrepareTest`
  (bind _asbp_third_person_character (cast `/Game/ThirdPerson/Blueprints/BP_ThirdPersonCharacter` (`GameplayStatics.GetPlayerCharacter` 0)))
  (set `self.Dimples` _asbp_third_person_character))

(event `self.ReceiveStartTest`
  (bind _dimples (`self.Dimples`))
  (set `/Game/ThirdPerson/Blueprints/BP_ThirdPersonCharacter.Health` 100 _dimples)
  (`/Game/ThirdPerson/Blueprints/BP_ThirdPersonCharacter.Increase_Health` _dimples)
  (`self.AssertTrue` (`/Game/ThirdPerson/Blueprints/BP_ThirdPersonCharacter.Alive` _dimples))
  (if true
    (`self.FinishTest` "Succeeded" "You're alive!")
    (else
      (`self.FinishTest` "Failed" "You're somehow dead already"))))

(fn `UserConstructionScript`)