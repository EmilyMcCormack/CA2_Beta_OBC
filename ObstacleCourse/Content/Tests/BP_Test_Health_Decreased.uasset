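; Functional test that checks the third-person character's DecreaseHealth function lowers Health by the expected amount.
; PrepareTest casts the first player's character to BP_ThirdPersonCharacter and stores it as Dimples.
; StartTest seeds a known Health, calls DecreaseHealth, asserts the resulting integer, and finishes the test as succeeded or failed with a message.
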(event `self.ReceivePrepareTest`
  (bind _asbp_third_person_character (cast `/Game/ThirdPerson/Blueprints/BP_ThirdPersonCharacter` (`GameplayStatics.GetPlayerCharacter` 0)))
  (set `self.Dimples` _asbp_third_person_character))

(event `self.ReceiveStartTest`
  (bind _dimples (`self.Dimples`))
  (set `/Game/ThirdPerson/Blueprints/BP_ThirdPersonCharacter.Health` 75 _dimples)
  (`/Game/ThirdPerson/Blueprints/BP_ThirdPersonCharacter.Decrease_Health` _dimples)
  (bind _returnvalue (`self.AssertValue_Int` (`/Game/ThirdPerson/Blueprints/BP_ThirdPersonCharacter.Health` _dimples) "Equal_To" 25))
  (if _returnvalue
    (`self.FinishTest` "Succeeded" "Health Decreased!")
    (else
      (`self.FinishTest` "Failed" "Health NOT decreased"))))

(fn `UserConstructionScript`)